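; Player HUD for a timed-run game that owns the Timer, MainMenu and LevelSelect widgets, all created and hidden at BeginPlay.
; Bound dispatchers drive begin run, end run, main menu and overlay toggle, switching widget visibility, cursor and input mode.
; The overlay swaps timer for menu and blocks move input, while a separate toggle swaps menu and level select.
; Display text and high score resets forward to the Timer.
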(event `DisplayText`
  (params (NewParam :type Text))
  (`/Game/Blueprints/HUD/Timer.DisplayTextEvent` (stale `self.ReceiveBeginPlay` _returnvalue) NewParam))

(event `self.ReceiveBeginPlay`
  (add `self.EndRunDispatcher` (delegate `EndRun`))
  (add `self.BeginRunDispatcher` (delegate `BeginGame`))
  (add `self.MainMenuDispatcher` (delegate `MainMenu`))
  (add `self.ToggleOverlayDispatcher` (delegate `ToggleOverlay`))
  (bind _returnvalue (`|CreateWidget` "/Game/Blueprints/HUD/Timer.Timer_C"))
  (`UserWidget.AddToViewport` _returnvalue 0)
  (bind _returnvalue_2 (`|CreateWidget` "/Game/Blueprints/HUD/MainMenu.MainMenu_C"))
  (`UserWidget.AddToViewport` _returnvalue_2 0)
  (set `self.MainMenuRef` _returnvalue_2)
  (bind _returnvalue_3 (`|CreateWidget` "/Game/Blueprints/HUD/LevelSelect.LevelSelect_C"))
  (bind _output_get (set `self.LevelSelectRef` _returnvalue_3))
  (`UserWidget.AddToViewport` _output_get 0)
  (`Widget.SetVisibility` _returnvalue "Hidden")
  (`Widget.SetVisibility` _returnvalue_2 "Hidden")
  (`Widget.SetVisibility` _returnvalue_3 "Hidden"))

(event `BeginGame`
  (bind _returnvalue (`GameplayStatics.GetPlayerController` 0))
  (`Widget.SetVisibility` (stale `self.ReceiveBeginPlay` _returnvalue_2) "Visible")
  (`Widget.SetVisibility` (stale `self.ReceiveBeginPlay` _returnvalue) "Visible")
  (`Widget.SetVisibility` (stale `self.ReceiveBeginPlay` _returnvalue_2) "Hidden")
  (`/Game/Blueprints/HUD/Timer.StartRun` (stale `self.ReceiveBeginPlay` _returnvalue))
  (set `PlayerController.bShowMouseCursor` false _returnvalue)
  (`WidgetBlueprintLibrary.SetInputMode_GameOnly` _returnvalue))

(event `EndRun`
  (`/Game/Blueprints/HUD/Timer.EndRun` (stale `self.ReceiveBeginPlay` _returnvalue)))

(event `MainMenu`
  (bind _returnvalue (`GameplayStatics.GetPlayerController` 0))
  (`Widget.SetVisibility` (stale `self.ReceiveBeginPlay` _returnvalue_2) "Visible")
  (set `PlayerController.bShowMouseCursor` true _returnvalue)
  (`WidgetBlueprintLibrary.SetInputMode_UIOnlyEx` _returnvalue))

(event `ToggleOverlay`
  (bind _returnvalue (`GameplayStatics.GetPlayerController` 0))
  (if (`self.IsOverlayShowing`)
    (`Widget.SetVisibility` (stale `self.ReceiveBeginPlay` _returnvalue) "Visible")
    (`Widget.SetVisibility` (stale `self.ReceiveBeginPlay` _returnvalue_2) "Hidden")
    (`WidgetBlueprintLibrary.SetInputMode_GameOnly` _returnvalue)
    (`Controller.SetIgnoreMoveInput` _returnvalue false)
    (set `PlayerController.bShowMouseCursor` false _returnvalue)
    (set `self.IsOverlayShowing` false)
    (else
      (`Widget.SetVisibility` (stale `self.ReceiveBeginPlay` _returnvalue_2) "Visible")
      (`Widget.SetVisibility` (stale `self.ReceiveBeginPlay` _returnvalue) "Hidden")
      (`WidgetBlueprintLibrary.SetInputMode_GameAndUIEx` _returnvalue)
      (`Controller.SetIgnoreMoveInput` _returnvalue true)
      (set `PlayerController.bShowMouseCursor` true _returnvalue)
      (set `self.IsOverlayShowing` true))))

(event `ToggleLevelSelect`
  (bind _levelselectref (`self.LevelSelectRef`))
  (if (`self.IsLevelSelectShowing`)
    (`Widget.SetVisibility` (stale `self.ReceiveBeginPlay` _returnvalue_2) "Visible")
    (`Widget.SetVisibility` (`self.MainMenuRef`) "Visible")
    (`Widget.SetVisibility` _levelselectref "Hidden")
    (set `self.IsLevelSelectShowing` false)
    (else
      (`Widget.SetVisibility` _levelselectref "Visible")
      (`Widget.SetVisibility` (`self.MainMenuRef`) "Hidden")
      (set `self.IsLevelSelectShowing` true))))

(event `ResetHighScore`
  (`/Game/Blueprints/HUD/Timer.Reset High Score` (stale `self.ReceiveBeginPlay` _returnvalue)))

(fn `UserConstructionScript`)